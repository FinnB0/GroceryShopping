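; BP_ItemSpawner is an actor that randomly scatters copies of a chosen item class across a grid when play begins.
; Nested loops over X and Y give each cell a low, fixed-weight random chance to spawn ItemToSpawn.
; Grid spacing offsets from the spawner's location along world axes, while items inherit its rotation plus a ZRotation yaw offset.
; A leftover index comparison branch never runs, and the construction script is empty.
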(event `self.ReceiveBeginPlay`
  (bind (_returnvalue_roll _returnvalue_pitch _returnvalue_yaw) (`KismetMathLibrary.BreakRotator` (`self.K2_GetActorRotation`)))
  (for _index (range (+ (`self.X`) 1))
    (for _index_2 (range (+ (`self.Y`) 1))
      (if (`KismetMathLibrary.RandomBoolWithWeight` 0.1)
        (`|SpawnActorFromClass` (`self.ItemToSpawn`) (`KismetMathLibrary.MakeTransform` (+ (`KismetMathLibrary.MakeVector` (* _index (`self.X_Space`)) (* _index_2 (`self.Y_Space`))) (`self.K2_GetActorLocation`)) (`KismetMathLibrary.MakeRotator` _returnvalue_roll _returnvalue_pitch (+ _returnvalue_yaw (`self.Z_Rotation`)))) "Undefined" "MultiplyWithRoot" null null)))))

(fn `UserConstructionScript`)