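; BP_Shelf is a shelf actor that labels itself with an item name and stocks itself with pickups of that item at BeginPlay.
; It looks up the item in DT_Items by ShelfStructs.ItemIndex, spawning nothing if the row is missing.
; At each of five arrow components it fills a centered, world-axis XY grid with BP_PickUpItem actors, using weighted random gaps and slight yaw jitter for variety.
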(event `self.ReceiveBeginPlay`
  (bind (_returnvalue_roll _returnvalue_pitch _returnvalue_yaw) (`KismetMathLibrary.BreakRotator` (`self.K2_GetActorRotation`)))
  (bind ((`X_Amount_2_6B9ABD244553B607649A38854B430924` _x_amount) (`Y_Amount_4_B2888D8844B566A9C0C2AFA990F97216` _y_amount) (`X_Space_7_C79325824B3C40D76142A58531FEEB0A` _x_space) (`Y_Space_9_08C1184C4E1B9C423C7685A09EB24D53` _y_space) (`Z_Rotation_15_4905F8204A72F03F179062A1BAEED103` _z_rotation)) (break `/Game/Blueprints/ShelfStruct` (`self.ShelfStructs`)))
  (bind (_itemproperties _bitemexists) (`self.Create Item`))
  (if _bitemexists
    (`self.SetDisplayText` (`.Name_2_777C91A146A858BC519DA496B3A62D90` (break `/Game/Blueprints/ItemStruct` _itemproperties)))
    (for _array_element (`|MakeArray` (`self.Arrow1`) (`self.Arrow2`) (`self.Arrow3`) (`self.Arrow4`) (`self.Arrow`))
      (for _index (range 1 (+ _x_amount 1))
        (for _index_2 (range 1 (+ _y_amount 1))
          (if (`KismetMathLibrary.RandomBoolWithWeight` (`self.SpawnPossibility`))
            (`|SpawnActorFromClass` "/Game/Blueprints/BP_PickUpItem.BP_PickUpItem_C" (`KismetMathLibrary.MakeTransform` (+ (`KismetMathLibrary.MakeVector` (* _index _x_space) (* _index_2 _y_space)) (`SceneComponent.K2_GetComponentLocation` _array_element) (`KismetMathLibrary.MakeVector` (* (* _x_amount _x_space) -0.5) (* (* _y_amount _y_space) -0.5))) (`KismetMathLibrary.MakeRotator` _returnvalue_roll _returnvalue_pitch (+ _returnvalue_yaw _z_rotation (`KismetMathLibrary.RandomFloatInRange` -5.0 5.0)))) "Undefined" "MultiplyWithRoot" null _itemproperties null)))))))

(fn `Create Item`
  (returns (ItemProperties :type "/Game/Blueprints/ItemStruct Structure") (bItemExists :type Boolean))
  (bind _returnvalue (`|GetDataTableRow` "/Game/Blueprints/DT_Items.DT_Items" (`KismetStringLibrary.Conv_StringToName` (`KismetStringLibrary.Conv_IntToString` (`.ItemIndex_12_E4C5B54F42C318D456FF4EA66BA05433` (break `/Game/Blueprints/ShelfStruct` (`self.ShelfStructs`))))))
    (:`then`
      (return _returnvalue true))
    (:`RowNotFound`
      (return (struct) false))))

(fn `SetDisplayText`
  (params (Name :type Text))
  (`TextRenderComponent.K2_SetText` (`self.TextRender`) Name))

(fn `UserConstructionScript`)