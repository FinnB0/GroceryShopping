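; Mimic enemy that disguises itself as a nearby pickup item and chases the player when undisguised.
; A looping morph cycle sphere-traces for a BP_PickUpItem, copies its mesh onto a gravity-enabled MorphMesh, then pops back with a timeline scale-up of the skeletal mesh.
; Once a sphere overlap spots the player, Tick pushes and rotates it toward the camera unless morphed or stunned.
; Damage triggers a brief retriggerable stun.
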(event `Morph`
  (bind _returnvalue (`self.K2_GetActorLocation`))
  (bind _morphmesh (`self.MorphMesh`))
  (set `self.bIsMorphed` true)
  (bind _outhit (`KismetSystemLibrary.SphereTraceSingleForObjects` :`Start` _returnvalue :`End` _returnvalue :`Radius` 1000.0 :`ObjectTypes` (`|MakeArray` "ObjectTypeQuery4" :!type "EObjectTypeQuery Enum") :`DrawDebugType` "ForDuration"))
  (bind _asbp_pick_up_item (cast `/Game/Blueprints/BP_PickUpItem` (`.HitActor` (`GameplayStatics.BreakHitResult` _outhit)))
    (:`then`
      (`StaticMeshComponent.SetStaticMesh` _morphmesh (`.ItemMesh_10_C935F23A432CF17513D918ADD8EDE64F` (break `/Game/Blueprints/ItemStruct` (`/Game/Blueprints/BP_PickUpItem.ItemStruct` _asbp_pick_up_item))))
      (`SceneComponent.SetHiddenInGame` _morphmesh false false)
      (`SceneComponent.SetHiddenInGame` (`self.SkeletalMesh`) true false)
      (`PrimitiveComponent.SetEnableGravity` (`self.MorphMesh`) true)
      (`KismetSystemLibrary.Delay` 10.0)
      (`self.UnMorph`))
    (:`CastFailed`
      (`KismetSystemLibrary.Delay` 10.0 :!label _label)
      (`self.Morph`))))

(event `self.ReceiveBeginPlay`
  (`self.CreateMI`)
  (`KismetSystemLibrary.Delay` 2.0)
  (`self.Morph`))

(event `UnMorph`
  (bind _morphmesh (`self.MorphMesh`))
  (`PrimitiveComponent.SetEnableGravity` _morphmesh false)
  (`PrimitiveComponent.AddImpulse` _morphmesh (0.0 0.0 50.0) "None" true)
  (`KismetSystemLibrary.Delay` 1.0)
  (`SceneComponent.SetHiddenInGame` (`self.MorphMesh`) true false)
  (`SceneComponent.SetWorldScale3D` (`self.SkeletalMesh`) (0.01 0.01 0.01))
  (`SceneComponent.SetHiddenInGame` (`self.SkeletalMesh`) false false)
  (bind (_direction _scaletrack) (`Timeline|UnMorphTimer`)
    (:`Update`
      (`SceneComponent.SetWorldScale3D` (`self.SkeletalMesh`) (`KismetMathLibrary.VLerp` (0.01 0.01 0.01) (0.15 0.15 0.15) _scaletrack)))
    (:`Finished`
      (`StaticMeshComponent.SetStaticMesh` (`self.MorphMesh`) "/Engine/BasicShapes/Sphere.Sphere")
      (set `self.bIsMorphed` false)
      (goto _label))))

(event `self.Sphere1.OnComponentBeginOverlap`
  (params (OverlappedComponent :type "PrimitiveComponent Object Reference") (OtherActor :type "Actor Object Reference") (OtherComp :type "PrimitiveComponent Object Reference") (OtherBodyIndex :type Integer) (bFromSweep :type Boolean) (SweepResult :type "HitResult Structure (by ref)"))
  (cast `/Game/Blueprints/BP_FirstPersonCharacter` OtherActor)
  (set `self.bSeesPlayer` true))

(event `self.ReceiveTick`
  (params (DeltaSeconds :type "Float (single-precision)"))
  (bind _returnvalue (`KismetMathLibrary.Normal` (- (`self.K2_GetActorLocation` (`GameplayStatics.GetPlayerCameraManager` 0)) (`self.K2_GetActorLocation`))))
  (if (and (`self.bSeesPlayer`) (not (`self.bIsStunned?`)) (not (`self.bIsMorphed`)))
    (`PrimitiveComponent.AddForce` (`self.MorphMesh`) (* _returnvalue (`self.Speed`)) "None" true)
    (`self.K2_SetActorRotation` (`KismetMathLibrary.RInterpTo` (`self.K2_GetActorRotation`) (`KismetMathLibrary.MakeRotFromX` _returnvalue) 0.25 0.1))))

(event `/Game/Blueprints/BPI_Interaction.Damage`
  (set `self.bIsStunned?` true)
  (`KismetSystemLibrary.RetriggerableDelay` 3.0)
  (set `self.bIsStunned?` false))

(fn `CreateMI`
  (bind _skeletalmesh (`self.SkeletalMesh`))
  (bind _returnvalue (`PrimitiveComponent.CreateDynamicMaterialInstance` _skeletalmesh 0 (`PrimitiveComponent.GetMaterial` _skeletalmesh 0) "None"))
  (set `self.MI_Mimic` _returnvalue))

(fn `ShowDetails`
  (returns (Name :type Text) (Subtitle :type Text) (ButtonInfo :type Text) (bHasInfo :type Boolean))
  (return "" "" "" false))

(fn `UserConstructionScript`)