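; Blueprint function library that converts a time value into display text in minutes:seconds:hundredths form.
; TimeToText derives each field by truncation and modulo on the raw time in seconds, takes absolute values, and joins them with colons.
; Minutes wrap at 60 with no hours field, and the sign of negative times is dropped.
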(fn `TimeToText`
  (params (Time :type "Float (double-precision)"))
  (returns (Text :type Text))
  (return (`KismetTextLibrary.Conv_StringToText` (`KismetStringLibrary.Concat_StrStr` (`KismetTextLibrary.Conv_TextToString` (`KismetTextLibrary.Conv_IntToText` (`KismetMathLibrary.Abs_Int` (mod (`KismetMathLibrary.FTrunc` (/ Time 60.0)) 60)) false true 2)) ":" (`KismetTextLibrary.Conv_TextToString` (`KismetTextLibrary.Conv_IntToText` (`KismetMathLibrary.Abs_Int` (mod (`KismetMathLibrary.FTrunc` Time) 60)) false true 2)) ":" (`KismetTextLibrary.Conv_TextToString` (`KismetTextLibrary.Conv_IntToText` (`KismetMathLibrary.Abs_Int` (mod (`KismetMathLibrary.FTrunc` (* Time 100.0)) 100)) false true 2))))))