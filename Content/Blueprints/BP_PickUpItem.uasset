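; Pickup item actor that takes its mesh, material, name and cost from an item struct and shows a grab prompt.
; Interacting sphere-traces toward the camera to push physics items in between aside, notifies the player pawn, then hides the item without destroying it.
; Overlaps enable physics and nudge it by the other actor's velocity.
; Damage destroys it, while Reset restores its start transform, collision and visibility.
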(event `self.ReceiveBeginPlay`
  (`self.InitItem`)
  (set `self.StartTransform` (`self.GetTransform`)))

(event `/Game/Blueprints/BPI_Interaction.Interact`
  ;[1 1 1] Add Impulse to Items between Camera and this Item
  (bind _outhits (`KismetSystemLibrary.SphereTraceMultiForObjects` (`self.K2_GetActorLocation`) (`PlayerCameraManager.GetCameraLocation` (`GameplayStatics.GetPlayerCameraManager` 0)) 2.0 (`|MakeArray` "ObjectTypeQuery4" :!type "EObjectTypeQuery Enum")))
  (for _array_element _outhits
    (bind (_bblockinghit _binitialoverlap _time _distance _location _impactpoint _normal _impactnormal _physmat _hitactor _hitcomponent _hitbonename _bonename _hititem _elementindex _faceindex _tracestart _traceend) (`GameplayStatics.BreakHitResult` _array_element))
    (`PrimitiveComponent.SetSimulatePhysics` _hitcomponent true)
    (`PrimitiveComponent.AddImpulse` _hitcomponent (* (`KismetMathLibrary.Normal` (- _traceend _tracestart)) 100.0) "None" true))
  (message `/Game/Blueprints/BPI_Shopping.ItemPicked` (`GameplayStatics.GetPlayerPawn` 0) (`self.ItemStruct`))
  (`PrimitiveComponent.SetSimulatePhysics` (`self.Cube`) false)
  (`PrimitiveComponent.SetCollisionEnabled` (`self.Cube`) "NoCollision")
  (`self.SetActorHiddenInGame` true))

(event `self.Cube.OnComponentBeginOverlap`
  (params (OverlappedComponent :type "PrimitiveComponent Object Reference") (OtherActor :type "Actor Object Reference") (OtherComp :type "PrimitiveComponent Object Reference") (OtherBodyIndex :type Integer) (bFromSweep :type Boolean) (SweepResult :type "HitResult Structure (by ref)"))
  (bind _cube (`self.Cube`))
  (`PrimitiveComponent.SetSimulatePhysics` _cube true)
  (`PrimitiveComponent.AddImpulse` _cube (* (`self.GetVelocity` OtherActor) 0.1) "None" false))

(event `/Game/Blueprints/BPI_Interaction.Damage`
  (`self.K2_DestroyActor`))

(event `/Game/Blueprints/BPI_Reset.Reset`
  (`PrimitiveComponent.SetSimulatePhysics` (`self.Cube`) false)
  (`self.K2_SetActorTransform` (`self.StartTransform`))
  (`PrimitiveComponent.SetCollisionEnabled` (`self.Cube`) "QueryAndPhysics")
  (`self.SetActorHiddenInGame` false))

(fn `InitItem`
  (bind _cube (`self.Cube`))
  (bind ((`ItemMesh_10_C935F23A432CF17513D918ADD8EDE64F` _itemmesh) (`OverrideMaterial_15_043892EB4C32953DA042199A05927215` _overridematerial)) (break `/Game/Blueprints/ItemStruct` (`self.ItemStruct`)))
  (`StaticMeshComponent.SetStaticMesh` _cube _itemmesh)
  (`/Engine/EditorBlueprintResources/StandardMacros.IsValid` _overridematerial
    (:`Is Valid`
      (`PrimitiveComponent.SetMaterial` _cube 0 _overridematerial))))

(fn `ShowDetails`
  (returns (Name :type Text) (Subtitle :type Text) (ButtonInfo :type Text) (bHasInfo :type Boolean))
  (bind ((`Name_2_777C91A146A858BC519DA496B3A62D90` _name) (`Costs_11_D9C3819E4834124C62BC81A11D46CB7D` _costs)) (break `/Game/Blueprints/ItemStruct` (`self.ItemStruct`)))
  (return _name (`KismetTextLibrary.Conv_StringToText` (`KismetStringLibrary.Concat_StrStr` (`KismetStringLibrary.Conv_IntToString` _costs) " ct")) "Press [E] to grab" true))

(fn `UserConstructionScript`)