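; A laser beam hazard that respawns a BP_FirstPersonCharacter on overlap with its box.
; The construction script uses Space to place the two emitter meshes, size the box and set the beam's end point.
; Damage permanently disables overlaps and hides the beam.
; Interacting before that respawns the player with a red "DON'T TOUCH!" HUD message, and ShowDetails supplies prompt text hinting to shoot it.
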(event `self.Box.OnComponentBeginOverlap`
  (params (OverlappedComponent :type "PrimitiveComponent Object Reference") (OtherActor :type "Actor Object Reference") (OtherComp :type "PrimitiveComponent Object Reference") (OtherBodyIndex :type Integer) (bFromSweep :type Boolean) (SweepResult :type "HitResult Structure (by ref)"))
  (bind _asbp_first_person_character (cast `/Game/Blueprints/BP_FirstPersonCharacter` OtherActor))
  (`/Game/Blueprints/BP_FirstPersonCharacter.Respawn` _asbp_first_person_character))

(event `/Game/Blueprints/BPI_Interaction.Damage`
  (set `PrimitiveComponent.bGenerateOverlapEvents` false (`self.Box`))
  (`SceneComponent.SetHiddenInGame` (`self.LaserBeam`) true false)
  (set `self.bIsDestroyed` true))

(event `/Game/Blueprints/BPI_Interaction.Interact`
  (if (not (`self.bIsDestroyed`))
    (bind _asbp_first_person_character (cast `/Game/Blueprints/BP_FirstPersonCharacter` (`GameplayStatics.GetPlayerPawn` 0)))
    (`/Game/Blueprints/BP_FirstPersonCharacter.Respawn` _asbp_first_person_character)
    (`/Game/Blueprints/Widgets/W_HUD.CreateMassage` (`/Game/Blueprints/BP_FirstPersonCharacter.W_HUD` _asbp_first_person_character) "DON'T TOUCH!" (struct :`R` 1.0 :`B` 0.1 :`A` 1.0))))

(fn `ShowDetails`
  (returns (Name :type Text) (Subtitle :type Text) (ButtonInfo :type Text))
  (return "Laser Beam" "Don't Touch!" "Shot to deactivate"))

(fn `UserConstructionScript`
  (bind _space (`self.Space`))
  (`SceneComponent.K2_SetRelativeLocation` (`self.LaserMesh2`) (`KismetMathLibrary.MakeVector` _space) false false)
  (`SceneComponent.K2_SetRelativeLocation` (`self.LaserMesh1`) (`KismetMathLibrary.MakeVector` (* _space -1.0)) false false)
  (`BoxComponent.SetBoxExtent` (`self.Box`) (`KismetMathLibrary.MakeVector` _space 5.0 5.0) true)
  (`FXSystemComponent.SetVectorParameter` (`self.LaserBeam`) "User.BeamEnd" (`SceneComponent.K2_GetComponentLocation` (`self.LaserMesh2`))))