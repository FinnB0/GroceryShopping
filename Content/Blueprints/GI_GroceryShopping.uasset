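; GI_GroceryShopping, a game instance by its name prefix, holds shared state for a grocery shopping game.
; It stores a shopping list, a time and an end time, each written through its own setter event.
; Getter functions return the shopping list and time, while the end time has only a setter.
; It contains no other logic, acting purely as a data holder.
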(event `/Game/Blueprints/BPI_GroceryShopping.SetShoppingList`
  (params (ShoppingList :type "Map of Integer to Integer"))
  (set `self.ShoppingList` ShoppingList))

(event `/Game/Blueprints/BPI_GroceryShopping.SetTime`
  (params (Time :type "Float (double-precision)"))
  (set `self.Time` Time))

(event `/Game/Blueprints/BPI_GroceryShopping.SetEndTime`
  (params (EndTime :type "Float (double-precision)"))
  (set `self.EndTime` EndTime))

(fn `GetShoppingList`
  (returns (ShoppingList :type "Map of Integer to Integer"))
  (return (`self.ShoppingList`)))

(fn `GetTime`
  (returns (Time :type "Float (double-precision)"))
  (return (`self.Time`)))