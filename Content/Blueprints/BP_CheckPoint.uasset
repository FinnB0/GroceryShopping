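; BP_CheckPoint is a checkpoint gate that registers itself with BP_FirstPersonCharacter via SetCheckPoint when the character overlaps its box.
; The construction script uses Space to position the two detector meshes and size the trigger between them.
; Both meshes share one dynamic material instance, so ToggleCheckPointLight switches them together between bright cyan (active) and dim red (inactive).
; It starts inactive, and nothing in this Blueprint activates the light.
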(event `self.ReceiveBeginPlay`
  (`self.ToggleCheckPointLight` false))

(event `self.Box.OnComponentBeginOverlap`
  (params (OverlappedComponent :type "PrimitiveComponent Object Reference") (OtherActor :type "Actor Object Reference") (OtherComp :type "PrimitiveComponent Object Reference") (OtherBodyIndex :type Integer) (bFromSweep :type Boolean) (SweepResult :type "HitResult Structure (by ref)"))
  (bind _asbp_first_person_character (cast `/Game/Blueprints/BP_FirstPersonCharacter` OtherActor))
  (`/Game/Blueprints/BP_FirstPersonCharacter.SetCheckPoint` _asbp_first_person_character self))

(fn `CreateMÌ`
  (bind _detectormesh1 (`self.DetectorMesh1`))
  (bind _returnvalue (`PrimitiveComponent.CreateDynamicMaterialInstance` _detectormesh1 1 (`PrimitiveComponent.GetMaterial` _detectormesh1 1) "None"))
  (bind _output_get (set `self.MI_DetectorLight` _returnvalue))
  (`PrimitiveComponent.SetMaterial` (`self.DetectorMesh2`) 1 _output_get))

(fn `ToggleCheckPointLight`
  (params (bIsActive :type Boolean))
  (bind _mi_detectorlight (`self.MI_DetectorLight`))
  (bind _mi_detectorlight_2 (`self.MI_DetectorLight`))
  (if bIsActive
    (`MaterialInstanceDynamic.SetVectorParameterValue` _mi_detectorlight_2 "EmissiveColor" (struct :`G` 0.8 :`B` 1.0 :`A` 1.0))
    (`MaterialInstanceDynamic.SetScalarParameterValue` _mi_detectorlight_2 "EmissiveAmount" 100.0)
    (else
      (`MaterialInstanceDynamic.SetVectorParameterValue` _mi_detectorlight "EmissiveColor" (struct :`R` 1.0 :`A` 1.0))
      (`MaterialInstanceDynamic.SetScalarParameterValue` _mi_detectorlight "EmissiveAmount" 1.0))))

(fn `UserConstructionScript`
  (bind _space (`self.Space`))
  (`SceneComponent.K2_SetRelativeLocation` (`self.DetectorMesh2`) (`KismetMathLibrary.MakeVector` _space) false false)
  (`SceneComponent.K2_SetRelativeLocation` (`self.DetectorMesh1`) (`KismetMathLibrary.MakeVector` (* _space -1.0)) false false)
  (`BoxComponent.SetBoxExtent` (`self.Box`) (`KismetMathLibrary.MakeVector` _space 200.0 600.0) true)
  (`self.CreateMÌ`))