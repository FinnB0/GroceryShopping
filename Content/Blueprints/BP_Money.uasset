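; BP_Money is a collectible coin pickup that awards its Value to the player.
; Interact, Damage, or overlap by BP_FirstPersonCharacter all collect it, hiding the mesh, disabling its collision and sending CollectMoneyMessage to player pawn 0.
; Reset restores the mesh and returns the actor to the transform saved at BeginPlay.
; ShowDetails supplies the coin amount and collect prompt text for display.
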(event `self.ReceiveBeginPlay`
  (set `self.StartTransform` (`self.GetTransform`)))

(event `/Game/Blueprints/BPI_Interaction.Interact`
  (bind _moneymesh (`self.MoneyMesh`))
  (`PrimitiveComponent.SetCollisionEnabled` _moneymesh "NoCollision" :!label _label)
  (`SceneComponent.SetHiddenInGame` _moneymesh true false)
  (message `/Game/Blueprints/BPI_Shopping.CollectMoney` (`GameplayStatics.GetPlayerPawn` 0) (`self.Value`)))

(event `/Game/Blueprints/BPI_Interaction.Damage`
  (goto _label))

(event `/Game/Blueprints/BPI_Reset.Reset`
  (bind _moneymesh (`self.MoneyMesh`))
  (`PrimitiveComponent.SetCollisionEnabled` _moneymesh "QueryOnly")
  (`SceneComponent.SetHiddenInGame` _moneymesh false false)
  (`self.K2_SetActorTransform` (`self.StartTransform`)))

(event `self.MoneyMesh.OnComponentBeginOverlap`
  (params (OverlappedComponent :type "PrimitiveComponent Object Reference") (OtherActor :type "Actor Object Reference") (OtherComp :type "PrimitiveComponent Object Reference") (OtherBodyIndex :type Integer) (bFromSweep :type Boolean) (SweepResult :type "HitResult Structure (by ref)"))
  (cast `/Game/Blueprints/BP_FirstPersonCharacter` OtherActor)
  (`/Game/Blueprints/BPI_Interaction.Interact`))

(fn `ShowDetails`
  (returns (Name :type Text) (Subtitle :type Text) (ButtonInfo :type Text) (bHasInfo :type Boolean))
  (return (`KismetTextLibrary.Conv_StringToText` (`KismetStringLibrary.Concat_StrStr` (`KismetStringLibrary.Conv_IntToString` (`self.Value`)) " Coins")) "Buy Stuff" "Press E to Collect" false))

(fn `UserConstructionScript`)